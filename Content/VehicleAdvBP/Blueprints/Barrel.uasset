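; Barrel is a destructible prop in the VehicleAdvBP folder that respawns after something overlaps it.
; On overlap it saves a transform from the Destructible component's relative location and rotation at unit scale.
; After a short delay it disables actor collision and enables gravity on the Destructible and Box components.
; After a longer delay it destroys itself and spawns a new Barrel at the saved transform.
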(event EventBeginPlay)

(event Collision|EventActorBeginOverlap
  (params (OtherActor :type Actor%20Object%20Reference))
  (bind _destructible (Variables|Default|GetDestructible))
  (Variables|Default|SetLocation (Math|Transform|MakeTransform (Variables|/Script/Engine.SceneComponent|GetRelativeLocation _destructible) (Variables|/Script/Engine.SceneComponent|GetRelativeRotation _destructible)))
  (Utilities|FlowControl|Delay 1.0)
  (Collision|SetActorEnableCollision false)
  (Physics|SetEnableGravity (Variables|Default|GetDestructible) true)
  (Utilities|FlowControl|Delay 5.0)
  (Actor|DestroyActor)
  (Game|SpawnActorfromClass "Barrel_C" (Variables|Default|GetLocation) "Undefined" 0 0))

(event EventTick
  (params (DeltaSeconds :type Float%20%28single-precision%29)))

(fn ConstructionScript)